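; Inventory container component that holds an array of item slots, treating an ItemId of 0 as empty.
; AddItem fills the first empty slot, then UpdateUI forwards player-inventory changes to the owner's player controller.
; Slot drag-and-drop is unfinished: DropSlot calls an empty HandleDrop, and Transfer only writes within its own array.
; AddItemToIndex ignores the passed item, writing the empty target slot back onto itself.
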(fn `AddItem`
  (params (AddItemInfo :type "/Game/_Main/Blueprints/Inventory/Structures/S_ItemInfo Structure"))
  (returns (AddResult :type Boolean))
  (locals (LocalIndex :type Integer :default 0))
  (bind (_array_index _isfindempty) (`self.FindEmptySlot`))
  (bind _localindex (`local.LocalIndex`))
  (set `local.LocalIndex` _array_index)
  (if _isfindempty
    (`KismetArrayLibrary.Array_Set` (`self.Items`) _localindex AddItemInfo)
    (`self.UpdateUI` _localindex AddItemInfo)
    (`KismetSystemLibrary.PrintString` (`KismetStringLibrary.Conv_IntToString` (`.ItemId_4_E143AD7F4A3B68D89C4112BAF536CCAD` (break `/Game/_Main/Blueprints/Inventory/Structures/S_ItemInfo` (`self.GetItemAtIndex` 0)))))
    (return true)
    (else
      (return false))))

(fn `AddItemToIndex`
  (params (FromIndx :type Integer) (ToIndex :type Integer) (ItemInfo :type "/Game/_Main/Blueprints/Inventory/Structures/S_ItemInfo Structure"))
  (returns (Result :type Boolean))
  (if (`self.IsSlotEmpty` ToIndex)
    (`KismetArrayLibrary.Array_Set` (`self.Items`) ToIndex (`self.GetItemAtIndex` ToIndex))
    (return true)
    (else
      (return false))))

(fn `DropSlot`
  (params (DragIndex :type Integer) (DropIndex :type Integer) (FromContainerComp :type "/Game/_Main/Blueprints/Inventory/BPC_ItemsContainer Object Reference"))
  (`self.Handle Drop` DragIndex DropIndex FromContainerComp))

(fn `FindEmptySlot`
  (returns (`Array Index` :type Integer) (IsFindEmpty :type Boolean))
  (locals (IsFind :type Boolean))
  (for (_array_element _array_index) (`self.Items`)
    (if (== (`.ItemId_4_E143AD7F4A3B68D89C4112BAF536CCAD` (break `/Game/_Main/Blueprints/Inventory/Structures/S_ItemInfo` _array_element)) 0)
      (set `local.IsFind` true)
      (break)))
  (return _array_index (`local.IsFind`)))

(fn `GetItemAtIndex`
  (params (Index :type Integer))
  (returns (Item :type "/Game/_Main/Blueprints/Inventory/Structures/S_ItemInfo Structure"))
  (bind _items (`self.Items`))
  (if (`KismetArrayLibrary.Array_IsValidIndex` _items)
    (return (`|GetArrayItem` _items Index))
    (else
      (return))))

(fn `Handle Drop`
  (params (DragIndex :type Integer) (DropIndex :type Integer) (FromContainerComp :type "/Game/_Main/Blueprints/Inventory/BPC_ItemsContainer Object Reference")))

(fn `IsSlotEmpty`
  (params (Index :type Integer))
  (returns (IsEmpty :type Boolean))
  (return (== (`.ItemId_4_E143AD7F4A3B68D89C4112BAF536CCAD` (break `/Game/_Main/Blueprints/Inventory/Structures/S_ItemInfo` (`self.GetItemAtIndex` Index))) 0)))

(fn `Transfer`
  (params (DragIndex :type Integer) (DropIndex :type Integer) (ToContainerComp :type "/Game/_Main/Blueprints/Inventory/BPC_ItemsContainer Object Reference"))
  (`/Engine/EditorBlueprintResources/StandardMacros.IsValid` ToContainerComp
    (:`Is Valid`
      (`self.AddItemToIndex` DragIndex DropIndex (`self.GetItemAtIndex` DragIndex))
      (return))))

(fn `UpdateUI`
  (params (Index :type Integer) (ItemInfo :type "/Game/_Main/Blueprints/Inventory/Structures/S_ItemInfo Structure") (IsResetSlot :type Boolean))
  (bind _containertype (`self.ContainerType`))
  (if (not IsResetSlot)
    (switch `/Game/_Main/Blueprints/Inventory/Enum/E_ContainerType` _containertype
      (:`NewEnumerator0`
        (bind _survivalpcref (message `/Game/_Main/Blueprints/Inventory/I_SurvivialCharacter.GetPcFromCharacter` (`self.GetOwner`)))
        (`/Game/_Main/Blueprints/Inventory/PC_Survival.UpdateUI` _survivalpcref Index ItemInfo _containertype)))))