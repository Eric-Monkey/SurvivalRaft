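; Player inventory component, a child of a base container component, that manages item slots and keeps the inventory UI in sync.
; InitInventory fills the slots with empty item entries, and HandleDrop has the source container transfer to this one, only when the source is a Player Inventory.
; AddItemToIndex and ClearItemAtIndex overrides call the parent, then on success trigger UI updates, with adds reaching the player controller through the owning character.
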(fn `AddItemToIndex`
  (params (FromIndx :type Integer) (ToIndex :type Integer) (ItemInfo :type "/Game/_Main/Blueprints/Inventory/Structures/S_ItemInfo Structure"))
  (bind _result (`parent.AddItemToIndex` FromIndx ToIndex ItemInfo))
  (if _result
    (bind _survivalpcref (message `/Game/_Main/Blueprints/Inventory/I_SurvivialCharacter.GetPcFromCharacter` (`self.GetOwner`)))
    (`/Game/_Main/Blueprints/Inventory/PC_Survival.UpdateUI` _survivalpcref ToIndex ItemInfo (`self.ContainerType`))))

(fn `ClearItemAtIndex`
  (params (index :type Integer))
  (returns (isClear :type Boolean))
  (bind _isclear (`parent.ClearItemAtIndex` index))
  (if _isclear
    (`self.Update UI` index (struct) true)))

(fn `Handle Drop`
  (params (DragIndex :type Integer) (DropIndex :type Integer) (FromContainerComp :type "/Game/_Main/Blueprints/Inventory/BPC_ItemsContainer Object Reference"))
  (locals (LocalDragIndex :type Integer :default 0) (LocalDropIndex :type Integer :default 0))
  (set `local.LocalDragIndex` DragIndex)
  (set `local.LocalDropIndex` DropIndex)
  (`/Engine/EditorBlueprintResources/StandardMacros.IsValid` FromContainerComp
    (:`Is Valid`
      (switch `/Game/_Main/Blueprints/Inventory/Enum/E_ContainerType` (`/Game/_Main/Blueprints/Inventory/BPC_ItemsContainer.ContainerType` FromContainerComp)
        (:`NewEnumerator0`
          (`self.Transfer` FromContainerComp (`local.LocalDragIndex`) (`local.LocalDropIndex`) self))))))

(fn `InitInventory`
  (for _ (range (`self.InventorySize`))
    (`KismetArrayLibrary.Array_Add` (`self.Items`) (make `/Game/_Main/Blueprints/Inventory/Structures/S_ItemInfo` 0 0 false 0 null "" null))))