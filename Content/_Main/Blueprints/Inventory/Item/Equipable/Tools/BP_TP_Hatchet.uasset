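; Equippable hatchet tool actor that chops harvestable objects and awards their resources to the owning character.
; Use plays first- and third-person chop montages behind a swing lock; the anim notify has the client send a harvest location to the server.
; The server sphere-overlaps there with debug drawing, damaging each hit actor.
; Depleted targets pass their DT_HarvestList resources to the character's server harvest call, then expire.
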(event `Overlay_OnServer`
  (params (Location :type "Vector Structure"))
  (`self.Overlap` Location))

(event `/Game/_Main/Blueprints/Inventory/BPI_Item.UseItem`
  (bind _returnvalue (`self.GetOwner`))
  (if (not (`self.IsSwing`))
    (set `self.IsSwing` true)
    (message `/Game/_Main/Blueprints/Inventory/BPI_SurvivialCharacter.PlayMontageFP` _returnvalue "/Game/Man/Animation/Hatchet_Chop_Montage.Hatchet_Chop_Montage")
    (message `/Game/_Main/Blueprints/Inventory/BPI_SurvivialCharacter.PlayMontageTP` _returnvalue "/Game/Man/Animation/Hatchet_Chop_Montage.Hatchet_Chop_Montage")))

(event `/Game/_Main/Blueprints/Inventory/BPI_Equipable.UseAnimEnd`
  (set `self.IsSwing` false))

(event `/Game/_Main/Blueprints/Inventory/BPI_Equipable.UseAnimNotify`
  (`self.GetHarvestLocation_OnClient`))

(event `GetHarvestLocation_OnClient`
  (bind _harvestloc (message `/Game/_Main/Blueprints/Inventory/BPI_SurvivialCharacter.GetHarvestLocation` (`self.GetOwner`)))
  (`self.Overlay_OnServer` _harvestloc))

(fn `Do Harvest`
  (params (HarvestRef :type "Actor Object Reference"))
  (returns (Resources :type "Array of /Game/_Main/Struct/Harvest/S_Resource Structure"))
  (locals (LocLarteItemRef :type "Actor Object Reference") (LocCharRef :type "Actor Object Reference"))
  (set `local.LocLarteItemRef` HarvestRef)
  (bind _ref (message `/Game/_Main/Blueprints/Harvest/BPI_LargeItem.GetRef` (`local.LocLarteItemRef`)))
  (bind _returnvalue (`|GetDataTableRow` "/Game/_Main/DataTable/Harvest/DT_HarvestList.DT_HarvestList" (`/Game/_Main/Blueprints/Harvest/BP_HarvestMaster.HarvestID` _ref))
    (:`then`
      (return (`.Resources_6_874B2B824BE1250704F58B9EBA54E1F7` (break `/Game/_Main/Struct/Harvest/S_HarvestInfo` _returnvalue))))
    (:`RowNotFound`
      (return))))

(fn `GetEquipableRef`
  (returns (EquipableRef :type "/Game/_Main/Blueprints/Inventory/Item/Equipable/BP_EquipableMaster Object Reference"))
  (return self))

(fn `Overlap`
  (params (Location :type "Vector Structure"))
  (locals (HitObjectType :type "Array of EObjectTypeQuery Enum") (IgnoreActors :type "Array of Actor Object Reference"))
  (bind (_outactors _returnvalue) (`KismetSystemLibrary.SphereOverlapActors` Location 60.0 (`|MakeArray` "ObjectTypeQuery8" :!type "EObjectTypeQuery Enum") null (`|MakeArray` (`self.GetOwner`))))
  (`KismetSystemLibrary.DrawDebugSphere` (0.0 0.0 0.0) 60.0 12 (struct :`R` 1.0 :`G` 0.43372 :`B` 0.159859 :`A` 1.0) 10.0 1.0)
  (if _returnvalue
    (`KismetSystemLibrary.PrintString` "hit Tree")
    (for _array_element _outactors
      (bind _health (message `/Game/_Main/Blueprints/Harvest/BPI_LargeItem.ChangeHealth` _array_element 20.0))
      (if (<= _health 0.0)
        (`|ExecutionSequence`
          (:`then_0`
            (bind _resources (`self.Do Harvest` _array_element))
            (bind _survivalref (message `/Game/_Main/Blueprints/Inventory/BPI_SurvivialCharacter.GetCharacterRef` (`self.GetOwner`)))
            (`/Game/_Main/Player/BP_FirstPersonCharacter.HarvestOnServer` _survivalref _resources))
          (:`then_1`
            (`self.SetLifeSpan` _array_element 0.1)))))
    (else
      (`KismetSystemLibrary.PrintString` "False"))))

(fn `UserConstructionScript`
  (`parent.UserConstructionScript`))