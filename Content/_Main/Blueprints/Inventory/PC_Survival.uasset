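; Player controller for a survival game that owns the main UI for inventory, hotbar and harvest notifications.
; On BeginPlay without authority it creates the main widget, shows the cursor and runs a HUD string test.
; Tab toggles the inventory, switching cursor and input mode.
; Events update or clear inventory and hotbar slots by index and container type, or add harvested items to the notification list.
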(event `self.ReceiveBeginPlay`
  (if (not (`self.HasAuthority`))
    (bind _returnvalue (`|CreateWidget` "/Game/_Main/Blueprints/Inventory/Widget/UMG_Main.UMG_Main_C"))
    (bind _output_get (set `self.MainUI` _returnvalue))
    (`UserWidget.AddToViewport` _output_get 0)
    (set `self.bShowMouseCursor` true)
    (`self.Test`)))

(event `Key|Tab`
  (params (Key :type "Key Structure"))
  (:`Pressed`
    (`self.LocalInventoryVis`)))

(event `LocalInventoryVis`
  (bind _mainui (`self.MainUI`))
  (if (`self.IsInventoryVis`)
    (`/Game/_Main/Blueprints/Inventory/Widget/UMG_Main.InventoryVis` _mainui false)
    (set `self.bShowMouseCursor` false)
    (`WidgetBlueprintLibrary.SetInputMode_GameOnly` self)
    (set `self.IsInventoryVis` false)
    (else
      (`/Game/_Main/Blueprints/Inventory/Widget/UMG_Main.InventoryVis` _mainui true)
      (set `self.bShowMouseCursor` true)
      (`WidgetBlueprintLibrary.SetInputMode_GameAndUIEx` self null)
      (set `self.IsInventoryVis` true))))

(event `UpdateUI`
  (params (Index :type Integer) (ItemInfo :type "/Game/_Main/Blueprints/Inventory/Structures/S_ItemInfo Structure") (ContainerType :type "/Game/_Main/Enum/E_ContainerType Enum" :default "NewEnumerator0"))
  (bind _mainui (`self.MainUI`))
  (switch `/Game/_Main/Enum/E_ContainerType` ContainerType
    (:`NewEnumerator0`
      (`/Game/_Main/Blueprints/Inventory/Widget/UMG_InventorySlot.Init Slot` (`|GetArrayItem` (`/Game/_Main/Blueprints/Inventory/Widget/UMG_ItemContainerGrid.Slots` (`/Game/_Main/Blueprints/Inventory/Widget/UMG_Inventory.UMG_ItemContainerGrid` (`/Game/_Main/Blueprints/Inventory/Widget/UMG_Main.UMG_Inventory` _mainui))) Index) ItemInfo false))
    (:`NewEnumerator1`
      (`/Game/_Main/Blueprints/Inventory/Widget/UMG_InventorySlot.Init Slot` (`|GetArrayItem` (`/Game/_Main/Blueprints/Inventory/Widget/UMG_ItemContainerGrid.Slots` (`/Game/_Main/Blueprints/Inventory/Widget/UMG_HotBar.UMG_ItemContainerGrid` (`/Game/_Main/Blueprints/Inventory/Widget/UMG_Main.UMG_HotBar` _mainui))) Index) ItemInfo false))))

(event `ClearUI`
  (params (Index :type Integer) (ContainerType :type "/Game/_Main/Enum/E_ContainerType Enum" :default "NewEnumerator0"))
  (switch `/Game/_Main/Enum/E_ContainerType` ContainerType
    (:`NewEnumerator0`
      (`/Game/_Main/Blueprints/Inventory/Widget/UMG_InventorySlot.Init Slot` :`self` (`|GetArrayItem` (`/Game/_Main/Blueprints/Inventory/Widget/UMG_ItemContainerGrid.Slots` (`/Game/_Main/Blueprints/Inventory/Widget/UMG_Inventory.UMG_ItemContainerGrid` (`/Game/_Main/Blueprints/Inventory/Widget/UMG_Main.UMG_Inventory` (`self.MainUI`)))) Index) :`IsClear` true))
    (:`NewEnumerator1`
      (`/Game/_Main/Blueprints/Inventory/Widget/UMG_InventorySlot.Init Slot` :`self` (`|GetArrayItem` (`/Game/_Main/Blueprints/Inventory/Widget/UMG_ItemContainerGrid.Slots` (`/Game/_Main/Blueprints/Inventory/Widget/UMG_HotBar.UMG_ItemContainerGrid` (`/Game/_Main/Blueprints/Inventory/Widget/UMG_Main.UMG_HotBar` (`self.MainUI`)))) Index) :`IsClear` true))))

(event `HarvestShow_OnServer`
  (params (ItemId :type Name) (Quantity :type Integer))
  (`/Game/_Main/Widget/UMG_HarvestShow.AddToShowList` (`/Game/_Main/Blueprints/Inventory/Widget/UMG_Main.UMG_HarvestShow` (`self.MainUI`)) ItemId Quantity))

(event `Test`
  (bind _astest_hud (cast `/Game/_Main/Blueprints/Test_HUD` (`self.GetHUD` self))
    (:`then`
      (`KismetSystemLibrary.PrintString` (`/Game/_Main/Blueprints/Test_HUD.TestString` _astest_hud)))
    (:`CastFailed`
      (`KismetSystemLibrary.PrintString` "Cast Fail"))))

(fn `GetPc`
  (returns (SurvivalPc :type "/Game/_Main/Blueprints/Inventory/PC_Survival Object Reference"))
  (return self))

(fn `UserConstructionScript`)