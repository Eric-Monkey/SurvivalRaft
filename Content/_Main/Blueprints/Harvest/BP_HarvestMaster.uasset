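; BP_HarvestMaster is the base Blueprint for harvestable objects, reading its resource yields and DesClass from DT_LargeItemHarvest by HarvestID.
; GetResources scales each row resource's base quantity by random multipliers for tool tier and preferred-type match, keeping entries that pass an above-zero check.
; That check re-evaluates the random math, so it can differ from the stored quantity.
; GetRef returns the instance itself.
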(fn ConstructionScript)

(fn GetResources
  (params (Tier :type E_ToolTier%20Enum :default "NewEnumerator0") (Type :type E_ToolType%20Enum :default "NewEnumerator3"))
  (bind _returnvalue (Utilities|GetDataTableRow "/Game/_Main/DataTable/Harvest/DT_LargeItemHarvest.DT_LargeItemHarvest" (Variables|Default|GetHarvestID))
    (:then
      (for _array_element (.Resources (Utilities|Struct|BreakS_HarvestInfo _returnvalue))
        (bind _structout (Utilities|Struct|SetmembersinS_Resource _array_element (Math|Float|Truncate (|(((Base*SeverRate)*TypeRate)*TierRate) (Math|Conversions|ToFloat(Integer) (.Quantity (Utilities|Struct|BreakS_Resource _array_element))) 1.0 (select (Utilities|Enum|Equal(Enum) (.PreferredType (Utilities|Struct|BreakS_Resource _array_element)) Type) (Math|Random|RandomFloatinRange 0.9 1.2) (Math|Random|RandomFloatinRange 0.1 0.5)) (Utilities|Select :Index Tier :NewEnumerator0 (Math|Random|RandomFloatinRange 1.0 1.5) :NewEnumerator1 (Math|Random|RandomFloatinRange 1.5 2.0))))))
        (if (> (Math|Float|Truncate (|(((Base*SeverRate)*TypeRate)*TierRate) (Math|Conversions|ToFloat(Integer) (.Quantity (Utilities|Struct|BreakS_Resource _array_element))) 1.0 (select (Utilities|Enum|Equal(Enum) (.PreferredType (Utilities|Struct|BreakS_Resource _array_element)) Type) (Math|Random|RandomFloatinRange 0.9 1.2) (Math|Random|RandomFloatinRange 0.1 0.5)) (Utilities|Select :Index Tier :NewEnumerator0 (Math|Random|RandomFloatinRange 1.0 1.5) :NewEnumerator1 (Math|Random|RandomFloatinRange 1.5 2.0)))) 0)
          (Utilities|Array|Add (LocalVariables|GetLoc_TempResources) _structout)))
      (return (LocalVariables|GetLoc_TempResources)))))

(fn GetDesClass
  (bind _returnvalue (Utilities|GetDataTableRow "/Game/_Main/DataTable/Harvest/DT_LargeItemHarvest.DT_LargeItemHarvest" (Variables|Default|GetHarvestID))
    (:then
      (return (.DesClass (Utilities|Struct|BreakS_HarvestInfo _returnvalue))))))

(fn GetRef
  (return self))