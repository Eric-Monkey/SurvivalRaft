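; BP_GroundBase is a base actor for harvestable ground items, defined by a HarvestID row in DT_GroundItemHarvest.
; GetResources reads that row's resource list, scales each quantity through a rate formula and returns entries above zero.
; All rates are fixed at 1.0, so Tier and Type have no effect, and the random tier and type multipliers are unconnected.
; Other getters expose the row's DesClass and the actor itself.
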(event EventBeginPlay
  (|CallParentFunction) ; 此节点被禁用，将不会被调用。\n从引脚连出引线来编译功能。
)

(event Collision|EventActorBeginOverlap
  (params (OtherActor :type Actor%20Object%20Reference))
  (|CallParentFunction OtherActor) ; 此节点被禁用，将不会被调用。\n从引脚连出引线来编译功能。
)

(event EventTick
  (params (DeltaSeconds :type Float%20%28single-precision%29))
  (|CallParentFunction DeltaSeconds) ; 此节点被禁用，将不会被调用。\n从引脚连出引线来编译功能。
)

(fn ConstructionScript
  (|CallParentFunction))

(fn GetResources
  (params (Tier :type E_ToolTier%20Enum :default "NewEnumerator0") (Type :type E_ToolType%20Enum :default "NewEnumerator3"))
  (bind _returnvalue (Utilities|GetDataTableRow "/Game/_Main/DataTable/Harvest/DT_GroundItemHarvest.DT_GroundItemHarvest" (Variables|Default|GetHarvestID))
    (:then
      (for _array_element (.Resources (Utilities|Struct|BreakS_HarvestInfo _returnvalue))
        (bind _structout (Utilities|Struct|SetmembersinS_Resource _array_element (Math|Float|Truncate (|(((Base*SeverRate)*TypeRate)*TierRate) (Math|Conversions|ToFloat(Integer) (.Quantity (Utilities|Struct|BreakS_Resource _array_element))) 1.0 1.0 1.0))))
        (if (> (Math|Float|Truncate (|(((Base*SeverRate)*TypeRate)*TierRate) (Math|Conversions|ToFloat(Integer) (.Quantity (Utilities|Struct|BreakS_Resource _array_element))) 1.0 1.0 1.0)) 0)
          (Utilities|Array|Add (LocalVariables|GetLoc_TempResources) _structout)))
      (return (LocalVariables|GetLoc_TempResources)))))

(fn GetDesClass
  (bind _returnvalue (Utilities|GetDataTableRow "/Game/_Main/DataTable/Harvest/DT_GroundItemHarvest.DT_GroundItemHarvest" (Variables|Default|GetHarvestID))
    (:then
      (return (.DesClass (Utilities|Struct|BreakS_HarvestInfo _returnvalue))))))

(fn GetHarvestGroundRef
  (return self))