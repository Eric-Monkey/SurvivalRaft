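; BP_WhirPool is a whirlpool hazard actor that moves between two points defined in DT_PointList.
; Init reads radius, speed, wait and damage data, then scales the actor to that radius.
; Timers start and stop projectile-movement travel based on distance over speed, snapping to the endpoint.
; The cylinder tracks overlapping actors, but damage only prints a message and its looping timers are unconnected.
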(event `self.ReceiveTick`
  (params (DeltaSeconds :type "Float (single-precision)"))
  (if (>= (`self.Delta Seconds`) (`self.Temp`))
    (set `self.Delta Seconds` 0.0)
    (`self.Move` (`self.BeginPointID`) (`self.EndPointID`))
    (else
      (set `self.Delta Seconds` (+ (`self.Delta Seconds`) DeltaSeconds)))))

(event `self.ReceiveBeginPlay`
  (`/Engine/EditorBlueprintResources/ActorMacros.Switch Has Authority`
    (:`Authority`
      _)
    (:`Remote`
      _))
  (`self.Move_OnServer` (`self.BeginPointID`) (`self.EndPointID`)))

(event `Move_OnServer`
  (params (BeginPoint :type Name) (NextPoint :type Name))
  (`self.Move` BeginPoint NextPoint))

(event `Move`
  (params (BeginPointId :type Name) (EndPointId :type Name))
  (`self.Init` BeginPointId EndPointId)
  (bind _returnvalue (`KismetSystemLibrary.K2_SetTimerDelegate` (delegate `BeginMove`) (`self.WaitTime`)))
  (set `self.WaitTimerHandle` _returnvalue))

(event `BeginMove`
  (`KismetSystemLibrary.K2_ClearAndInvalidateTimerHandle` (`self.WaitTimerHandle`))
  (bind _needsecond (`self.GetNeedSecond`))
  (`SceneComponent.K2_SetWorldLocation` (`self.Scene`) (`self.BeginPoint`) false false)
  (`self.SetSpeend` (`self.Speed`) (`self.GetMoveDirection`))
  (bind _returnvalue (`KismetSystemLibrary.K2_SetTimerDelegate` (delegate `StopMove`) _needsecond))
  (set `self.StopMoveTimerHandle` _returnvalue))

(event `StopMove`
  (`KismetSystemLibrary.K2_ClearAndInvalidateTimerHandle` (`self.StopMoveTimerHandle`))
  (`self.SetSpeend` (`self.Speed`))
  (`SceneComponent.K2_SetWorldLocation` (`self.Scene`) (`self.NextPoint`) false false))

(event `SetRadius`
  (params (Radius :type "Float (double-precision)") (Second :type "Float (double-precision)"))
  (`SceneComponent.SetRelativeScale3D` (`self.Scene`) (`KismetMathLibrary.MakeVector` Radius Radius 500.0)))

(event `self.Cylinder.OnComponentBeginOverlap`
  (params (OverlappedComponent :type "PrimitiveComponent Object Reference") (OtherActor :type "Actor Object Reference") (OtherComp :type "PrimitiveComponent Object Reference") (OtherBodyIndex :type Integer) (bFromSweep :type Boolean) (SweepResult :type "HitResult Structure (by ref)"))
  (`KismetArrayLibrary.Array_AddUnique` (`self.Players`) OtherActor))

(event `TakeDamage_OnServer`
  (`self.TakeDamage`))

(event `self.Cylinder.OnComponentEndOverlap`
  (params (OverlappedComponent :type "PrimitiveComponent Object Reference") (OtherActor :type "Actor Object Reference") (OtherComp :type "PrimitiveComponent Object Reference") (OtherBodyIndex :type Integer))
  (`KismetArrayLibrary.Array_RemoveItem` (`self.Players`) OtherActor))

(fn `GetCurrentDirection`
  (returns (CurDirection :type "Vector Structure"))
  (return (`KismetMathLibrary.Normal` (`MovementComponent.Velocity` (`self.ProjectileMovement`)))))

(fn `GetDamage`
  (params (ID :type Name))
  (returns (Damage :type "Float (double-precision)"))
  (return 0.0))

(fn `GetMoveDirection`
  (returns (Direction :type "Vector Structure"))
  (return (`KismetMathLibrary.Normal` (- (`self.NextPoint`) (`self.BeginPoint`)) 1e-05)))

(fn `GetNeedSecond`
  (returns (NeedSecond :type "Float (double-precision)"))
  (return (/ (`KismetMathLibrary.Vector_Distance` (`self.NextPoint`) (`self.BeginPoint`)) (`self.Speed`))))

(fn `GetPointData`
  (params (ID :type Name))
  (returns (PointData :type "/Game/whirlpool/S_WhirPool Structure"))
  (bind _returnvalue (`|GetDataTableRow` "/Game/whirlpool/DT_PointList.DT_PointList" ID)
    (:`then`
      (return _returnvalue))))

(fn `GetPointId`
  (params (ID :type Name)))

(fn `GetPointLocation`
  (params (ID :type Name))
  (returns (NewParam :type "Vector Structure"))
  (`|GetDataTableRow` "/Game/whirlpool/DT_PointList.DT_PointList" ID
    (:`then`
      (return (0.0 0.0 0.0)))))

(fn `GetSpeed`
  (params (ID :type Name)))

(fn `Init`
  (params (BeginPointId :type Name) (NextPointId :type Name))
  (locals (NewLocalVar :type "/Game/whirlpool/S_WhirPool Structure"))
  (`|ExecutionSequence`
    (:`then_0`
      (set `self.BeginPointID` BeginPointId)
      (set `self.EndPointID` NextPointId))
    (:`then_1`
      (bind _pointdata (`self.GetPointData` BeginPointId))
      (bind ((`Location_22_84B0789C4AFC97CFC8E80A8BA6219A0B` _location) (`Radius_21_5279C84046D760E44CE4A088E667D386` _radius) (`Damage_12_B443EEA24DC094D2B68ACD872F1A70AE` _damage) (`Speed_31_5585D50449C0233BF32955A55A9408C8` _speed) (`WaitTime_24_D018168F4336C57DEE2A1FBCD0BFFD0D` _waittime) (`DamageCoolDown_30_A11607A644BADE412E928AAE417E230C` _damagecooldown)) (break `/Game/whirlpool/S_WhirPool` _pointdata))
      (set `self.BeginPoint` (`KismetMathLibrary.MakeVector` (.x _location) (.y _location)))
      (set `self.Radius` _radius)
      (set `self.Damage` _damage)
      (set `self.Speed` _speed)
      (set `self.WaitTime` _waittime)
      (set `self.CoolDown` _damagecooldown)
      (`self.SetSpeend` 0.0)
      (`self.SetRadius` (`self.Radius`)))
    (:`then_2`
      (bind _pointdata_2 (`self.GetPointData` NextPointId))
      (bind ((`Location_22_84B0789C4AFC97CFC8E80A8BA6219A0B` _location_2) (`Radius_21_5279C84046D760E44CE4A088E667D386` _radius_2)) (break `/Game/whirlpool/S_WhirPool` _pointdata_2))
      (set `self.NextPointRadius` _radius_2)
      (set `self.NextPoint` _location_2))))

(fn `SetSpeend`
  (params (Speed :type "Float (double-precision)") (Direction :type "Vector Structure"))
  (set `MovementComponent.Velocity` (* (`KismetMathLibrary.Normal` Direction) Speed) (`self.ProjectileMovement`)))

(fn `TakeDamage`
  (for _ (`self.Players`)
    (`KismetSystemLibrary.PrintString` (`KismetTextLibrary.Conv_TextToString` (`|FormatText` "makeDMG:{DMG}" (`self.Damage`))))))

(fn `UserConstructionScript`)

(fn `新函数_0`)